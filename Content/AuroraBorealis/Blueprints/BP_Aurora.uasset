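; Aurora borealis actor that displays a spline mesh with adjustable opacity and optional color overrides.
; The construction script assigns the chosen mesh, creates dynamic material instances, and applies starting opacity, colors and top-to-bottom ratio.
; A second underside material is used only when the mesh is the complex line variant.
; FadeIn and FadeOut play or reverse one rate-scaled timeline that drives SetOpacity, or set opacity instantly for non-positive durations.
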(event Custom|FadeIn
  (params (FadeTimeSeconds :type Float%20%28double-precision%29))
  (bind _fadeintimeline (Variables|Default|GetFadeInTimeline))
  ;[0 0 0] Fade In / Out
  (if (> FadeTimeSeconds 0.0)
    (Components|Timeline|SetPlayRate (Variables|Default|GetFadeInTimeline) (/ 1.0 FadeTimeSeconds))
    (if (Class|TimelineComponent|IsReversing (Variables|Default|GetFadeInTimeline))
      (Audio|Components|Audio|Play _fadeintimeline)
      (else
        (Components|Timeline|PlayfromStart _fadeintimeline)))
    (else
      (CallFunction|SetOpacity 1.0))))

(event Custom|FadeOut
  (params (FadeTimeSeconds :type Float%20%28double-precision%29))
  (bind _fadeintimeline (Variables|Default|GetFadeInTimeline))
  ;[0 0 0] Fade In / Out
  (if (> FadeTimeSeconds 0.0)
    (Components|Timeline|SetPlayRate (Variables|Default|GetFadeInTimeline) (/ 1.0 FadeTimeSeconds))
    (if (Audio|Components|Audio|IsPlaying (Variables|Default|GetFadeInTimeline))
      (Utilities|String|Reverse _fadeintimeline)
      (else
        (Components|Timeline|ReversefromEnd _fadeintimeline)))
    (else
      (CallFunction|SetOpacity 0.0))))

(fn ConstructionScript
  (bind _splinemesh (Variables|Default|GetSplineMesh))
  (bind _meshtouse (Variables|Appearance|GetMeshToUse))
  (Utilities|FlowControl|Sequence
    (:then_0
      ;[0 0 0] Assign the static mesh
      (Components|StaticMesh|SetStaticMesh (Variables|Default|GetSplineMesh) _meshtouse)
      (Variables|Private|SetHasUnderside (== _meshtouse "/Game/AuroraBorealis/Meshes/SM_Aurora_Line_Complex.SM_Aurora_Line_Complex")))
    (:then_1
      ;[0 0 0] Assign the dynamic material(s)
      (if (Variables|Private|GetHasUnderside)
        (bind _returnvalue (Rendering|Material|CreateDynamicMaterialInstance "/Game/AuroraBorealis/Materials/MI_AuroraBottom.MI_AuroraBottom" "None" "None" :!class /Script/Engine.KismetMaterialLibrary))
        (bind _output_get (Variables|Private|SetAuroraBottomDynMat _returnvalue))
        (Rendering|Material|SetMaterialbyName _splinemesh "AuroraUnderMat" _output_get)))
    (:then_2
      (bind _returnvalue_2 (Rendering|Material|CreateDynamicMaterialInstance "/Game/AuroraBorealis/Materials/MI_Aurora.MI_Aurora" "None" "None" :!class /Script/Engine.KismetMaterialLibrary))
      (bind _output_get_2 (Variables|Private|SetAuroraDynMat _returnvalue_2))
      (Rendering|Material|SetMaterialbyName _splinemesh "AuroraMat" _output_get_2))
    (:then_3
      ;[0 0 0] Override start opacity
      (CallFunction|SetOpacity (Variables|Appearance|GetStartOpacity)))
    (:then_4
      ;[0 0 0] Override start color
      (if (Variables|Appearance|Color|GetOverrideColor)
        (Rendering|Material|SetVectorParameterValue (Variables|Private|GetAuroraDynMat) "ColorTop" (Variables|Appearance|Color|GetTopColor) :!class /Script/Engine.MaterialInstanceDynamic)
        (Rendering|Material|SetVectorParameterValue (Variables|Private|GetAuroraDynMat) "ColorBottom" (Variables|Appearance|Color|GetBottomColor) :!class /Script/Engine.MaterialInstanceDynamic)
        (if (Variables|Private|GetHasUnderside)
          (Rendering|Material|SetVectorParameterValue (Variables|Private|GetAuroraBottomDynMat) "Color" (Variables|Appearance|Color|GetUnderColor) :!class /Script/Engine.MaterialInstanceDynamic))))
    (:then_5
      ;[0 0 0] Override top to bottom ratio
      (if (Variables|Appearance|Color|GetOverrideColor)
        (Rendering|Material|SetScalarParameterValue (Variables|Private|GetAuroraDynMat) "TopBottomRatio" (Variables|Appearance|Color|GetTopToBottomRatio) :!class /Script/Engine.MaterialInstanceDynamic)))))

(fn SetOpacity
  (params (NewOpacity :type Float%20%28double-precision%29))
  (Rendering|Material|SetScalarParameterValue (Variables|Private|GetAuroraDynMat) "Opacity" NewOpacity :!class /Script/Engine.MaterialInstanceDynamic)
  (if (Variables|Private|GetHasUnderside)
    (Rendering|Material|SetScalarParameterValue (Variables|Private|GetAuroraBottomDynMat) "Opacity" NewOpacity :!class /Script/Engine.MaterialInstanceDynamic))
  (return))