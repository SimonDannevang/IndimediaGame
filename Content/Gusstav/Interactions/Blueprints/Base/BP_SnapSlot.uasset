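; BP_SnapSlot is an interaction slot that snaps a passed-in actor into a set position and rotation.
; Snap clears the actor's Pawn reference, then moves its target component to the SnapTarget transform offset from the slot, keeping world scale.
; The location offset is added in world space, unrotated by the slot, while rotations are combined.
; After the move, physics simulation is switched off on the component if active.
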(event Custom|Snap
  (params (Actor :type BP%20Snappable%20Object%20Reference))
  (bind _returnvalue (Transformation|GetActorTransform))
  (bind _component (Default|GetTargetComponent Actor))
  (bind _component_2 (Default|GetTargetComponent Actor))
  (bind _snaptarget (Variables|Default|GetSnapTarget))
  (bind (_location _rotation) (Math|Transform|BreakTransform _snaptarget))
  (bind (_location_2 _rotation_2) (Math|Transform|BreakTransform _returnvalue))
  (Variables|/Game/Gusstav/Interactions/Blueprints/Base/BP_Grabbable.BP_Grabbable_C|SetPawn Actor 0)
  (Utilities|FlowControl|Sequence
    (:then_0
      (Transformation|SetWorldTransform _component_2 (Math|Transform|MakeTransform (+ _location _location_2) (Math|Rotator|CombineRotators _rotation _rotation_2) (Transformation|GetWorldScale _component_2)) false false))
    (:then_1
      (if (Physics|IsSimulatingPhysics _component "None")
        (bind _asprimitive_component (Utilities|Casting|CastToPrimitiveComponent _component))
        (Physics|SetSimulatePhysics _asprimitive_component false)))))

(fn ConstructionScript)