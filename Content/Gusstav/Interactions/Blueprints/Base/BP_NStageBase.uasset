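; BP_NStageBase is a base Blueprint for interactables that step through a configurable number of stages.
; When an interaction stops, a short press advances CurrentStage, while a hold of at least ReverseHoldLength steps it back.
; The stage is clamped between zero and Stages, so it never wraps.
; GetMapped converts the current stage linearly into a caller-supplied Low to High range.
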(event EventBeginPlay)

(event Collision|EventActorBeginOverlap
  (params (OtherActor :type Actor%20Object%20Reference)))

(event EventTick
  (params (DeltaSeconds :type Float%20%28single-precision%29)))

(event EventInteractStop
  (params (Pawn :type Pawn%20Object%20Reference) (Hit :type Hit%20Result%20Structure) (HoldLength :type Float%20%28double-precision%29))
  (Variables|Default|SetCurrentStage (Math|Integer|Clamp(Integer) (+ (Variables|Default|GetCurrentStage) (Math|Integer|SelectInt -1 1 (>= HoldLength (Variables|Default|GetReverseHoldLength)))) 0 (Variables|Default|GetStages))))

(fn ConstructionScript)

(fn GetMapped
  (params (Low :type Float%20%28double-precision%29) (High :type Float%20%28double-precision%29))
  (return (Math|Float|MapRangeClamped (Math|Conversions|ToFloat(Integer) (Variables|Default|GetCurrentStage)) 0.0 (Math|Conversions|ToFloat(Integer) (Variables|Default|GetStages)) Low High)))