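; Base laser emitter actor that, while active, traces from its arrow component along its forward direction each tick to find what the beam hits.
; It tracks the hit actor as its target, sending laser start and stop messages when that changes and tick messages while it stays valid.
; Deactivation or a missed trace releases the target, and GetLaserSource exposes the laser's frequency.
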(event EventTick
  (params (DeltaSeconds :type Float%20%28single-precision%29))
  (bind _arrow (Variables|Default|GetArrow))
  (bind _returnvalue (Transformation|GetWorldLocation _arrow))
  (if (Variables|Default|GetActive)
    (Utilities|FlowControl|Sequence
      (:then_0
        (bind (_outhit _returnvalue_2) (Collision|LineTraceByChannel _returnvalue (+ _returnvalue (* (Math|Rotator|GetRotationXVector (Transformation|GetWorldRotation _arrow)) (Variables|Default|GetLaserDistance))) "TraceTypeQuery1" false 0 "None"))
        (bind _output_get (Variables|Default|SetLastHit _outhit))
        (if _returnvalue_2
          (if (not (== (Variables|Default|GetTarget) (.HitActor (Collision|BreakHitResult _output_get))))
            (Utilities|FlowControl|Sequence
              (:then_0
                (Class|BILaserTarget|LaserStop(Message) (Variables|Default|GetTarget) self :!label _label)
                (Variables|Default|SetTarget 0))
              (:then_1
                (bind _output_get_2 (Variables|Default|SetTarget (.HitActor (Collision|BreakHitResult _output_get))))
                (Class|BILaserTarget|LaserStart(Message) _output_get_2 self))))
          (else
            (goto _label))))
      (:then_1
        (Utilities|IsValid (Variables|Default|GetTarget)
          (:Is%20Valid
            (Class|BILaserTarget|LaserTick(Message) (Variables|Default|GetTarget) self DeltaSeconds)))))
    (else
      (Utilities|IsValid (Variables|Default|GetTarget)
        (:Is%20Valid
          (Class|BILaserTarget|LaserStop(Message) (Variables|Default|GetTarget) self)
          (Variables|Default|SetTarget 0))))))

(fn ConstructionScript)

(fn GetLaserSource
  (return (Variables|Default|GetFrequency)))