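; BP_WheelTransform is a base Blueprint that moves and rotates a component in proportion to a Percent value, presumably from a wheel interaction.
; The construction script caches the component's original relative transform.
; Each Tick eases it toward that original plus the completion offsets scaled by Percent, using delta-time lerps and shortest-path rotation.
; GetTransformComponent returns nothing here, leaving child classes to supply the component.
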(event EventBeginPlay)

(event Collision|EventActorBeginOverlap
  (params (OtherActor :type Actor%20Object%20Reference)))

(event EventTick
  (params (DeltaSeconds :type Float%20%28single-precision%29))
  (bind _returnvalue (* DeltaSeconds 2.0))
  (bind _percent (Variables|Default|GetPercent))
  (bind _originaltransform (Variables|Default|GetOriginalTransform))
  (bind (_location _rotation) (Math|Transform|BreakTransform _originaltransform))
  (|CallParentFunction DeltaSeconds)
  (Transformation|SetRelativeLocationAndRotation (CallFunction|GetTransformComponent) (Math|Vector|Lerp(Vector) (Variables|/Script/Engine.SceneComponent|GetRelativeLocation (CallFunction|GetTransformComponent)) (+ _location (* (Variables|Default|GetCompleteLocationTransform) _percent)) _returnvalue) (Math|Rotator|Lerp(Rotator) (Variables|/Script/Engine.SceneComponent|GetRelativeRotation (CallFunction|GetTransformComponent)) (Math|Rotator|CombineRotators (* (Variables|Default|GetCompleteRotationTransform) _percent) _rotation) _returnvalue true) false false))

(fn ConstructionScript
  (Variables|Default|SetOriginalTransform (Transformation|GetRelativeTransform (CallFunction|GetTransformComponent)))
  (|CallParentFunction))

(fn GetTransformComponent
  (return 0))