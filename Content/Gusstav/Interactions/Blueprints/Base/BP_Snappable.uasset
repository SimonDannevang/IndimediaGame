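; BP_Snappable is a base interactable Blueprint for snappable objects that manages the physics state of its target component.
; The construction script caches whether that component simulates physics in NeedPhysics.
; When an interaction starts, it runs the parent logic, then sets physics simulation on the component back to the cached value.
; Any snapping behavior itself is not in this graph.
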(event EventBeginPlay
  (|CallParentFunction) ; This node is disabled and will not be called.\nDrag off pins to build functionality.
)

(event Collision|EventActorBeginOverlap
  (params (OtherActor :type Actor%20Object%20Reference))
  (|CallParentFunction OtherActor) ; This node is disabled and will not be called.\nDrag off pins to build functionality.
)

(event EventTick
  (params (DeltaSeconds :type Float%20%28single-precision%29))
  (|CallParentFunction DeltaSeconds) ; This node is disabled and will not be called.\nDrag off pins to build functionality.
)

(event EventInteractStart
  (params (Pawn :type Pawn%20Object%20Reference) (Hit :type Hit%20Result%20Structure))
  (|CallParentFunction Pawn Hit)
  (bind _asprimitive_component (Utilities|Casting|CastToPrimitiveComponent (CallFunction|GetTargetComponent)))
  (Physics|SetSimulatePhysics _asprimitive_component (Variables|Default|GetNeedPhysics)))

(fn ConstructionScript
  (Variables|Default|SetNeedPhysics (Physics|IsSimulatingPhysics (CallFunction|GetTargetComponent) "None"))
  (|CallParentFunction))