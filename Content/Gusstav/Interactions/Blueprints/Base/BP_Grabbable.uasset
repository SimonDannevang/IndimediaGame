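; BP_Grabbable is a base interactable meant to let a third-person character hold and carry an object, but its logic is currently disconnected.
; InteractStart, InteractStop and Tick are empty, and GetTargetComponent returns nothing.
; The unwired graph traces along the pawn's hold ray, pulling the target via velocity when simulating physics, otherwise by lerping location.
; It also optionally turns the target with the camera and releases it beyond a drop distance.
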(event EventInteractStart
  (params (Pawn :type Pawn%20Object%20Reference) (Hit :type Hit%20Result%20Structure)))

(event EventTick
  (params (DeltaSeconds :type Float%20%28single-precision%29))
  ;[1 1 1] Basic Movement
)

(event EventInteractStop
  (params (Pawn :type Pawn%20Object%20Reference) (Hit :type Hit%20Result%20Structure) (HoldLength :type Float%20%28double-precision%29)))

(fn ConstructionScript)

(fn GetTargetComponent
  (return 0))