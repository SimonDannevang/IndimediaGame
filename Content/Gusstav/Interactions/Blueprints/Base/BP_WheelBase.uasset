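; Base Blueprint for a wheel interaction that accumulates a normalized progress value while being interacted with.
; Each interact tick moves Percent up or down by Speed, depending on the Reverse flag, clamped between zero and one.
; When interaction stops, ReverseOnStop optionally flips the direction for the next use.
; GetMapped remaps Percent to a caller-supplied range.
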(event EventInteractTick
  (params (Pawn :type Pawn%20Object%20Reference) (Hit :type Hit%20Result%20Structure) (Delta :type Float%20%28double-precision%29))
  (Variables|Default|SetPercent (Math|Float|Clamp(Float) (+ (Variables|Default|GetPercent) (* (* Delta (Variables|Default|GetSpeed)) (Math|Float|SelectFloat -1.0 1.0 (Variables|Default|GetReverse)))))))

(event EventInteractStop
  (params (Pawn :type Pawn%20Object%20Reference) (Hit :type Hit%20Result%20Structure) (HoldLength :type Float%20%28double-precision%29))
  (Variables|Default|SetReverse (Math|Boolean|NotEqual(Boolean) (Variables|Default|GetReverse) (Variables|Default|GetReverseOnStop))))

(fn ConstructionScript)

(fn GetMapped
  (params (Low :type Float%20%28double-precision%29) (High :type Float%20%28double-precision%29))
  (return (Math|Float|MapRangeClamped (Variables|Default|GetPercent) 0.0 1.0 Low High)))