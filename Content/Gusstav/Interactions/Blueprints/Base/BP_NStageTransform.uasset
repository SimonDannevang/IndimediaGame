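; Base interaction Blueprint that smoothly moves and rotates a component according to the actor's current stage.
; The construction script caches the component's relative transform as the origin.
; Each Tick eases the component toward that origin plus per-stage location and rotation offsets multiplied by CurrentStage, using delta-time lerps.
; GetTransformComponent returns nothing here, leaving child Blueprints to supply the component.
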(event EventBeginPlay
  (|CallParentFunction) ; This node is disabled and will not be called.\nDrag off pins to build functionality.
)

(event Collision|EventActorBeginOverlap
  (params (OtherActor :type Actor%20Object%20Reference))
  (|CallParentFunction OtherActor) ; This node is disabled and will not be called.\nDrag off pins to build functionality.
)

(event EventTick
  (params (DeltaSeconds :type Float%20%28single-precision%29))
  (bind _returnvalue (* DeltaSeconds 2.0))
  (bind _originaltransform (Variables|Default|GetOriginalTransform))
  (bind _currentstage (Variables|Default|GetCurrentStage))
  (bind (_location _rotation) (Math|Transform|BreakTransform _originaltransform))
  (|CallParentFunction DeltaSeconds)
  (Transformation|SetRelativeLocationAndRotation (CallFunction|GetTransformComponent) (Math|Vector|Lerp(Vector) (Variables|/Script/Engine.SceneComponent|GetRelativeLocation (CallFunction|GetTransformComponent)) (+ _location (* (Variables|Default|GetStageLocationTransform) _currentstage)) _returnvalue) (Math|Rotator|Lerp(Rotator) (Variables|/Script/Engine.SceneComponent|GetRelativeRotation (CallFunction|GetTransformComponent)) (Math|Rotator|CombineRotators (* (Variables|Default|GetStageRotationTransform) _currentstage) _rotation) _returnvalue true) false false))

(fn ConstructionScript
  (Variables|Default|SetOriginalTransform (Transformation|GetRelativeTransform (CallFunction|GetTransformComponent)))
  (|CallParentFunction))

(fn GetTransformComponent
  (return 0))