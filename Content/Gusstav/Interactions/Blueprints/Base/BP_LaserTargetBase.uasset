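; Base Blueprint for a laser target that becomes active or inactive as lasers of a matching frequency start and stop hitting it.
; LaserStart and LaserStop compare the source's message to TargetFrequency, then raise or lower a counter of matching sources.
; Active is true while that count is above zero, inverted when Reverse is set.
; LaserSnap returns a default of no end snapping and a zero location.
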(event EventLaserStart
  (params (Source :type Actor%20Object%20Reference))
  (bind _frequency (Class|BILaserSource|GetLaserSource(Message) Source))
  (if (== (Variables|Default|GetTargetFrequency) _frequency)
    (Math|Integer|IncrementInt (Variables|Default|GetSources)
      (:%20%20
        (Variables|Default|SetActive (Math|Boolean|NotEqual(Boolean) (> (Variables|Default|GetSources) 0) (Variables|Default|GetReverse)))))))

(event EventLaserStop
  (params (Source :type Actor%20Object%20Reference))
  (bind _frequency (Class|BILaserSource|GetLaserSource(Message) Source))
  (if (== (Variables|Default|GetTargetFrequency) _frequency)
    (Math|Integer|DecrementInt (Variables|Default|GetSources)
      (:%20%20
        (Variables|Default|SetActive (Math|Boolean|NotEqual(Boolean) (> (Variables|Default|GetSources) 0) (Variables|Default|GetReverse)))))))

(fn ConstructionScript)

(fn LaserSnap
  (return false "0, 0, 0"))