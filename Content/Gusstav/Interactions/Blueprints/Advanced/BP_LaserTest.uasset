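; BP_LaserTest is a laser Blueprint that draws its beam with a particle system, tinted by a Color parameter at construction.
; After the parent Tick, an active laser shows the beam, ending at the Target's snap location if requested, otherwise at the last hit's impact location or trace end.
; When inactive, it collapses the beam end to the Arrow and hides the particles.
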(event EventTick
  (params (DeltaSeconds :type Float%20%28single-precision%29))
  (bind _target (Variables|Default|GetTarget))
  (bind _lasthit (Variables|Default|GetLastHit))
  (bind (_bblockinghit _binitialoverlap _time _distance _location _impactpoint _normal _impactnormal _physmat _hitactor _hitcomponent _hitbonename _bonename _hititem _elementindex _faceindex _tracestart _traceend) (Collision|BreakHitResult _lasthit))
  (|CallParentFunction DeltaSeconds)
  (if (Variables|Default|GetActive)
    (Rendering|SetVisibility (Variables|Default|GetParticleSystem) true false)
    (Utilities|IsValid _target
      (:Is%20Valid
        (bind (_snapend _worldloc) (Class|BILaserTarget|LaserSnap(Message) _target))
        (if _snapend
          (Class|ParticleSystemComponent|SetBeamEndPoint (Variables|Default|GetParticleSystem) 0 _worldloc)
          (else
            (Class|ParticleSystemComponent|SetBeamEndPoint (Variables|Default|GetParticleSystem) 0 (Math|Vector|SelectVector _location _traceend _bblockinghit) :!label _label))))
      (:Is%20Not%20Valid
        (goto _label)))
    (else
      (Class|ParticleSystemComponent|SetBeamEndPoint (Variables|Default|GetParticleSystem) 0 (Transformation|GetWorldLocation (Variables|Default|GetArrow)))
      (Rendering|SetVisibility (Variables|Default|GetParticleSystem) false false))))

(fn ConstructionScript
  (|CallParentFunction)
  (Effects|Components|ParticleSystem|SetColorParameter (Variables|Default|GetParticleSystem) "Color" (Variables|Default|GetColor)))