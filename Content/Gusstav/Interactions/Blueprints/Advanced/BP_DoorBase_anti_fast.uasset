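; Door base Blueprint with two sliding panels that open and close according to an Opened flag.
; Every Tick lerps the left and right meshes' relative locations toward opposite Y offsets when Opened, or back to the origin when not.
; The delta-time-scaled alpha gives an eased slide without a timeline.
; Nothing in these graphs sets Opened, and movement does not sweep for collision.
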(event EventBeginPlay)

(event Collision|EventActorBeginOverlap
  (params (OtherActor :type Actor%20Object%20Reference)))

(event EventTick
  (params (DeltaSeconds :type Float%20%28single-precision%29))
  (bind _sm_door_left (Variables|Default|GetSM_Door_Left))
  (bind _sm_door_right (Variables|Default|GetSM_Door_Right))
  (Transformation|SetRelativeLocation _sm_door_left (Math|Vector|Lerp(Vector) (Variables|/Script/Engine.SceneComponent|GetRelativeLocation _sm_door_left) (Math|Vector|SelectVector "0,100.000000, 0" "0, 0, 0" (Variables|Default|GetOpened)) (* DeltaSeconds 5.0)) false false)
  (Transformation|SetRelativeLocation _sm_door_right (Math|Vector|Lerp(Vector) (Variables|/Script/Engine.SceneComponent|GetRelativeLocation _sm_door_right) (Math|Vector|SelectVector "0,-100.000000, 0" "0, 0, 0" (Variables|Default|GetOpened)) (* DeltaSeconds 5.0)) false false))

(fn ConstructionScript)