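; Test actor for a powered state, likely paired with a pressure interaction, that toggles a laser particle effect and sound from an Active flag.
; Tick polls Active and sets the particle system's visibility to match.
; Two cross-resetting DoOnce gates limit audio to state changes: activation spawns the laser sound at the actor with a fade-in, and deactivation fades it out.
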(event EventTick
  (params (DeltaSeconds :type Float%20%28single-precision%29))
  (bind _particlesystem (Variables|Default|GetParticleSystem))
  (if (Variables|Default|GetActive)
    (Rendering|SetVisibility _particlesystem true false)
    (Utilities|FlowControl|DoOnce false :!label _label
      (:Completed
        (bind _returnvalue (Audio|SpawnSoundatLocation "/Game/StarterContent/Audio/Laser_Cue.Laser_Cue" (Transformation|GetActorLocation) "0, 0, 0" 1.0 1.0 0.0 "/Game/Gusstav/SFX/LaserAttenuation.LaserAttenuation" 0))
        (Audio|Components|Audio|FadeIn _returnvalue 1.0 1.0 0.0 "Linear" :!class /Script/Engine.AudioComponent)
        (goto _label_2 Reset)))
    (else
      (Rendering|SetVisibility _particlesystem false false)
      (Utilities|FlowControl|DoOnce false :!label _label_2
        (:Completed
          (Utilities|IsValid _returnvalue
            (:Is%20Valid
              (Audio|Components|Audio|FadeOut _returnvalue 1.0 0.0 "Linear" :!class /Script/Engine.AudioComponent)
              (goto _label Reset))))))))

(fn ConstructionScript
  (|CallParentFunction))