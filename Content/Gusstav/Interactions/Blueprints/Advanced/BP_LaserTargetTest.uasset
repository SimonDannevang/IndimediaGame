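; Laser target actor that shows its active state with a colored point light and a looping-style laser sound cue.
; Tick syncs light visibility to Active and uses two cross-resetting DoOnce gates to fade the spawned sound in on activation and out on deactivation.
; The construction script applies Color to the light, and LaserSnap returns the SnapLaser setting with the Arrow's world location as a snap point.
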(event EventBeginPlay)

(event Collision|EventActorBeginOverlap
  (params (OtherActor :type Actor%20Object%20Reference)))

(event EventTick
  (params (DeltaSeconds :type Float%20%28single-precision%29))
  (|CallParentFunction DeltaSeconds)
  (Rendering|SetVisibility (Variables|Default|GetPointLight) (Variables|Default|GetActive) false)
  (if (Variables|Default|GetActive)
    (Utilities|FlowControl|DoOnce false :!label _label
      (:Completed
        (bind _returnvalue (Audio|SpawnSoundatLocation "/Game/StarterContent/Audio/Laser_Cue.Laser_Cue" (Transformation|GetActorLocation) "0, 0, 0" 1.0 1.0 0.0 "/Game/Gusstav/SFX/LaserAttenuation.LaserAttenuation" 0))
        (Audio|Components|Audio|FadeIn _returnvalue 1.0 1.0 0.0 "Linear" :!class /Script/Engine.AudioComponent)
        (goto _label_2 Reset)))
    (else
      (Utilities|FlowControl|DoOnce false :!label _label_2
        (:Completed
          (Utilities|IsValid _returnvalue
            (:Is%20Valid
              (Audio|Components|Audio|FadeOut _returnvalue 1.0 0.0 "Linear" :!class /Script/Engine.AudioComponent)
              (goto _label Reset))))))))

(fn ConstructionScript
  (|CallParentFunction)
  (Rendering|Components|Light|SetLightColor (Variables|Default|GetPointLight) (Variables|Default|GetColor) true))

(fn LaserSnap
  (return (Variables|Default|GetSnapLaser) (Transformation|GetWorldLocation (Variables|Default|GetArrow))))