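; BP_Smeltery is an interactive smeltery whose glow follows a temperature control.
; The construction script creates a dynamic glow material instance on one slot of the smeltery mesh, and BeginPlay starts its Intensity at zero.
; Each Tick, Temp eases toward the mapped TempControl value through a delta-time Lerp and drives that Intensity, so the glow changes gradually rather than snapping.
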(event EventBeginPlay
  (Rendering|Material|SetScalarParameterValue (Variables|Default|GetMat) "Intensity" 0.0 :!class /Script/Engine.MaterialInstanceDynamic))

(event Collision|EventActorBeginOverlap
  (params (OtherActor :type Actor%20Object%20Reference)))

(event EventTick
  (params (DeltaSeconds :type Float%20%28single-precision%29))
  (bind _output_get (Variables|Default|SetTemp (Math|Float|Lerp (Variables|Default|GetTemp) (Default|GetMapped (Variables|Default|GetTempControl) 0.0 5.0) DeltaSeconds)))
  (Rendering|Material|SetScalarParameterValue (Variables|Default|GetMat) "Intensity" _output_get :!class /Script/Engine.MaterialInstanceDynamic))

(fn ConstructionScript
  (bind _returnvalue (Rendering|Material|CreateDynamicMaterialInstance (Variables|Default|GetSM_Smeltery) 2 "/Game/Gusstav/Interactions/Materials/M_Smeltery_Glow.M_Smeltery_Glow" "None" :!class /Script/Engine.PrimitiveComponent))
  (Variables|Default|SetMat _returnvalue))