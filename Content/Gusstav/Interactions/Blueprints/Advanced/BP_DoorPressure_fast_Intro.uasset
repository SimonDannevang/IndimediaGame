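; Pressure-driven door for the intro, which mirrors its linked Pressure object's active state into Opened every Tick.
; The parent Tick runs after that update, then DoOnce gates limit the button-on sound as the state is polled.
; When inactive, it stops any valid on sound and handles the button-off sound, both spawned spatially at the door.
; A point light is visible only while Pressure is active.
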(event EventBeginPlay
  (|CallParentFunction) ; This node is disabled and will not be called.\nDrag off pins to build functionality.
)

(event Collision|EventActorBeginOverlap
  (params (OtherActor :type Actor%20Object%20Reference))
  (|CallParentFunction OtherActor) ; This node is disabled and will not be called.\nDrag off pins to build functionality.
)

(event EventTick
  (params (DeltaSeconds :type Float%20%28single-precision%29))
  (bind _pointlight (Variables|Default|GetPointLight))
  (Variables|Default|SetOpened (Variables|/Game/Gusstav/Interactions/Blueprints/Base/BP_PressureBase.BP_PressureBase_C|GetActive (Variables|Default|GetPressure)))
  (Utilities|FlowControl|Sequence
    (:then_0
      (|CallParentFunction DeltaSeconds))
    (:then_1
      (if (Variables|Default|GetOpened)
        (Utilities|FlowControl|DoOnce false :!label _label
          (:Completed
            (bind _returnvalue (Audio|SpawnSoundatLocation "/Game/Gusstav/SFX/Large_Button_Cue.Large_Button_Cue" (Transformation|GetActorLocation) "0, 0, 0" 1.0 1.0 0.0 "/Game/Gusstav/SFX/IntroLaserDoor_Attenuation.IntroLaserDoor_Attenuation" "/Game/Gusstav/SFX/NewSoundConcurrency_Axes.NewSoundConcurrency_Axes"))
            (goto _label_2 Reset)))
        (else
          (Utilities|FlowControl|Sequence
            (:then_0
              (goto _label Reset))
            (:then_1
              (Utilities|IsValid _returnvalue
                (:Is%20Valid
                  (Audio|Components|Audio|Stop _returnvalue))
                (:Is%20Not%20Valid
                  (Utilities|FlowControl|DoOnce false :!label _label_2
                    (:Completed
                      _))))
              (Audio|SpawnSoundatLocation "/Game/Gusstav/SFX/Large_Button_Cue_off.Large_Button_Cue_off" (Transformation|GetActorLocation) "0, 0, 0" 1.0 1.0 0.0 "/Game/Gusstav/SFX/IntroLaserDoor_Attenuation.IntroLaserDoor_Attenuation" "/Game/Gusstav/SFX/NewSoundConcurrency_Axes.NewSoundConcurrency_Axes"))))))
    (:then_2
      (if (Variables|/Game/Gusstav/Interactions/Blueprints/Base/BP_PressureBase.BP_PressureBase_C|GetActive (Variables|Default|GetPressure))
        (Rendering|SetVisibility _pointlight true false)
        (else
          (Rendering|SetVisibility _pointlight false false))))))

(fn ConstructionScript
  (|CallParentFunction))