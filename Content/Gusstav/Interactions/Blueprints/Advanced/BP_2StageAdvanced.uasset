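; Two-stage interaction Blueprint that animates a Lever component between an off pose and a completed pose based on the Switch flag.
; Each Tick it eases the Lever's relative location and shortest-path rotation toward the target, using DeltaSeconds times Speed as alpha.
; The completed pose offsets OriginalTransform by the configured location and rotation, while the off pose is relative zero rather than OriginalTransform.
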(event EventTick
  (params (DeltaSeconds :type Float%20%28single-precision%29))
  (bind _speed (Variables|Default|GetSpeed))
  (bind _originaltransform (Variables|Default|GetOriginalTransform))
  (bind (_location _rotation) (Math|Transform|BreakTransform _originaltransform))
  (bind _returnvalue (* DeltaSeconds _speed))
  (Transformation|SetRelativeLocationAndRotation (Variables|Default|GetLever) (Math|Vector|Lerp(Vector) (Variables|/Script/Engine.SceneComponent|GetRelativeLocation (Variables|Default|GetLever)) (Math|Vector|SelectVector (+ _location (Variables|Default|GetCompleteLocationTransform)) "0, 0, 0" (Variables|Default|GetSwitch)) _returnvalue) (Math|Rotator|Lerp(Rotator) (Variables|/Script/Engine.SceneComponent|GetRelativeRotation (Variables|Default|GetLever)) (Math|Rotator|SelectRotator (Math|Rotator|CombineRotators _rotation (Variables|Default|GetCompleteRotationTransform)) "0, 0, 0" (Variables|Default|GetSwitch)) _returnvalue true) false false))

(fn ConstructionScript
  (|CallParentFunction))