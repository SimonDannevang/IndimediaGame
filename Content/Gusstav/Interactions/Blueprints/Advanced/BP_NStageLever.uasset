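; BP_NStageLever is a multi-stage lever interaction actor that shows its current state as in-world text.
; It overrides GetTransformComponent to supply the Lever component as the transform component.
; Each Tick calls the parent, then writes CurrentStage and its GetMapped value over a symmetric range to a TextRender.
; Stage handling and mapping are not implemented in these graphs, which hold only this readout and the override.
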(event EventBeginPlay
  (|CallParentFunction) ; This node is disabled and will not be called.\nDrag off pins to build functionality.
)

(event Collision|EventActorBeginOverlap
  (params (OtherActor :type Actor%20Object%20Reference))
  (|CallParentFunction OtherActor) ; This node is disabled and will not be called.\nDrag off pins to build functionality.
)

(event EventTick
  (params (DeltaSeconds :type Float%20%28single-precision%29))
  (|CallParentFunction DeltaSeconds)
  (Rendering|Components|TextRender|SetText (Variables|Default|GetTextRender) (Utilities|Text|ToText(String) (Utilities|String|Append (Utilities|String|ToString(Integer) (Variables|Default|GetCurrentStage)) " -> " (Utilities|String|ToString(Float) (CallFunction|GetMapped -8.0 8.0))))))

(fn ConstructionScript
  (|CallParentFunction))

(fn GetTransformComponent
  (return (Variables|Default|GetLever)))