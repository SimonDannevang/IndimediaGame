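; BP_DoorLaser is a door driven by a laser target, setting its Opened state from whether that target is active.
; Each Tick it copies LaserTarget.Active into Opened, runs the parent Tick and toggles two point lights to match.
; A DoOnce plays the button-on sound once when opened, then on closing resets and stops that sound, playing the off sound if it is still valid.
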(event EventBeginPlay
  (|CallParentFunction) ; This node is disabled and will not be called.\nDrag off pins to build functionality.
)

(event Collision|EventActorBeginOverlap
  (params (OtherActor :type Actor%20Object%20Reference))
  (|CallParentFunction OtherActor) ; This node is disabled and will not be called.\nDrag off pins to build functionality.
)

(event EventTick
  (params (DeltaSeconds :type Float%20%28single-precision%29))
  (bind _pointlight (Variables|Default|GetPointLight))
  (bind _lasertarget (Variables|Default|GetLaserTarget))
  (bind _active (Variables|/Game/Gusstav/Interactions/Blueprints/Base/BP_LaserTargetBase.BP_LaserTargetBase_C|GetActive _lasertarget))
  (Variables|Default|SetOpened _active)
  (Utilities|FlowControl|Sequence
    (:then_0
      (|CallParentFunction DeltaSeconds))
    (:then_1
      (if _active
        (Rendering|SetVisibility _pointlight true false)
        (else
          (Rendering|SetVisibility _pointlight false false))))
    (:then_2
      (if (Variables|Default|GetOpened)
        (Utilities|FlowControl|DoOnce false :!label _label
          (:Completed
            (bind _returnvalue (Audio|SpawnSound2D "/Game/Gusstav/SFX/Large_Button_Cue.Large_Button_Cue" 1.0 1.0 0.0 0))))
        (else
          (Utilities|FlowControl|Sequence
            (:then_0
              (goto _label Reset))
            (:then_1
              (Utilities|IsValid _returnvalue
                (:Is%20Valid
                  (Audio|Components|Audio|Stop _returnvalue)
                  (Audio|SpawnSound2D "/Game/Gusstav/SFX/Large_Button_Cue_off.Large_Button_Cue_off" 1.0 1.0 0.0 0))))))))))

(fn ConstructionScript
  (|CallParentFunction))