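; BP_Temperature is an interaction Blueprint that shows a temperature readout in Kelvin.
; It overrides GetTransformComponent to supply the temperature arrow as the component for its parent class to work with.
; Each tick it runs the parent logic, gets the inherited value mapped onto a Kelvin range, truncates it and writes it to a text render with a K suffix.
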(event EventTick
  (params (DeltaSeconds :type Float%20%28single-precision%29))
  (|CallParentFunction DeltaSeconds)
  (Rendering|Components|TextRender|SetText (Variables|Default|GetTextRender) (Utilities|Text|ToText(String) (Utilities|String|Append (Utilities|String|ToString(Integer) (Math|Float|Truncate (CallFunction|GetMapped 0.0 3e+03))) " K"))))

(fn ConstructionScript
  (|CallParentFunction))

(fn GetTransformComponent
  (return (Variables|Default|GetSM_Temperature_Arrow)))