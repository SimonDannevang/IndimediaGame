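; BP_ItemSpawner_Statue_Intro is an item spawner that places a WeightedStatue at its own location and rotation.
; It attempts a spawn on BeginPlay and again when its Respawn event fires, after clearing CurrentItem and waiting DelayBeforeRespawn.
; AttemptToSpawn guards against duplicates through CurrentItem, but SpawnItem sets that variable to None instead of storing the new statue.
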(event EventBeginPlay
  (CallFunction|AttempttoSpawn))

(event EventRespawn
  (Variables|Default|SetCurrentItem 0)
  (Utilities|FlowControl|Delay (Variables|Default|GetDelayBeforeRespawn))
  (CallFunction|AttempttoSpawn))

(fn ConstructionScript)

(fn AttempttoSpawn
  (Utilities|IsValid (Variables|Default|GetCurrentItem)
    (:Is%20Valid
      (Development|PrintString "Item Already Spawned"))
    (:Is%20Not%20Valid
      (CallFunction|SpawnItem))))

(fn SpawnItem
  (Game|SpawnActorfromClass "/Game/Gusstav/Interactions/WeightedStatue.WeightedStatue_C" (Math|Transform|MakeTransform (Transformation|GetActorLocation) (Transformation|GetActorRotation)) "AdjustIfPossibleButAlwaysSpawn" self 0)
  (Variables|Default|SetCurrentItem 0))